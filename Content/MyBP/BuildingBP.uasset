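; Numbered building actor that lets the player blend the camera to it and back to the player pawn through widget buttons.
; On BeginPlay it sets its number label, hides its return widget and binds the SwitchCamera dispatchers of the fly-to and return buttons.
; Either switch hides return widgets on every BuildingBP instance.
; Flying to a building also starts a timer that reveals its return button as the blend ends.
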(event Custom|SwitchCamera_Event
  (Game|Player|SetViewTargetwithBlend (Game|GetPlayerController 0) self 4.0 "VTBlend_Linear" 0.0 false)
  (CallFunction|HideWidgetReturn)
  (Utilities|Time|SetTimerbyFunctionName 0 "ShowWidgetReturn" 4.0))

(event Custom|SwitchCamera_Event_0
  (Game|Player|SetViewTargetwithBlend (Game|GetPlayerController 0) (Game|Player|GetPlayerPawn 0) 4.0 "VTBlend_Linear" 0.0 false)
  (CallFunction|HideWidgetReturn))

(event EventBeginPlay
  (Rendering|Components|TextRender|SetText (Variables|Default|GetTextRender) (Utilities|Text|ToText(Name) (Variables|Default|GetNumber)))
  (Development|SetHiddeninGame (Variables|Default|GetWidgetReturn) true false)
  (bind _asbpw_button_return (Utilities|Casting|CastToBPW_ButtonReturn (UserInterface|GetWidget (Variables|Default|GetWidgetReturn))))
  (EventDispatchers|AssignSwitchCamera _asbpw_button_return (delegate Custom|SwitchCamera_Event_0))
  (bind _asbpw_button_to_fly (Utilities|Casting|CastToBPW_ButtonToFly (UserInterface|GetWidget (Variables|Default|GetWidgetToChose))))
  (EventDispatchers|AssignSwitchCamera _asbpw_button_to_fly (delegate Custom|SwitchCamera_Event)))

(fn ConstructionScript)

(fn ShowWidgetReturn
  (Development|SetHiddeninGame (Variables|Default|GetWidgetReturn) false false))

(fn HideWidgetReturn
  (bind _outactors (Actor|GetAllActorsOfClass "BuildingBP_C"))
  (for _array_element _outactors
    (Development|SetHiddeninGame (Variables|BuildingBP_C|GetWidgetReturn _array_element) true false)))