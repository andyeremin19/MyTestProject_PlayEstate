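; ManBP is a selectable playable character with a button widget for choosing it from among the placed ManBP actors.
; It binds the widget button's dispatcher on BeginPlay; selection destroys the current pawn, possesses this character, switches to game-only input, hides the widget and removes the other ManBP instances.
; Axis inputs drive movement and camera yaw, while SwitchState flip-flops the walk speed between fast and slow.
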(event Custom|MyDispatcher_Event
  (bind _returnvalue (Game|GetPlayerController 0))
  (bind _returnvalue_2 (Game|GetPlayerController 0))
  ;[1 1 1] Выбор персонажа
  (Actor|DestroyActor (Game|Player|GetPlayerPawn 0))
  (Input|SetInputModeGameOnly _returnvalue false)
  (Variables|/Script/Engine.PlayerController|SetbShowMouseCursor _returnvalue false)
  (Pawn|UnPossess _returnvalue_2)
  (Pawn|Possess _returnvalue_2 self)
  (Development|SetHiddeninGame (Variables|Default|GetWidget) true true)
  (bind _outactors (Actor|GetAllActorsOfClass "ManBP_C"))
  (for _array_element _outactors
    (if (Utilities|Enum|NotEqual(Enum) (Utilities|GetObjectName _array_element) (Utilities|GetObjectName self))
      (Actor|DestroyActor _array_element))))

(event EventBeginPlay
  ;[1 1 1] Выбор персонажа
  (bind _asbpw_button (Utilities|Casting|CastToBPW_Button (UserInterface|GetWidget (Variables|Default|GetWidget))))
  (bind _output_get (Variables|Default|SetAs%20BPW%20Button _asbpw_button))
  (EventDispatchers|AssignMyDispatcher _output_get (delegate Custom|MyDispatcher_Event)))

(event Input|ActionEvents|InputActionSwitchState
  (params (Key :type Key%20Structure :default "None"))
  (bind _charactermovement (Variables|Character|GetCharacterMovement))
  ;[1 1 1] Movement
  (:Pressed
    (Utilities|FlowControl|FlipFlop
      (:A
        (Variables|/Script/Engine.CharacterMovementComponent|SetMaxWalkSpeed _charactermovement 3e+02))
      (:B
        (Variables|/Script/Engine.CharacterMovementComponent|SetMaxWalkSpeed _charactermovement 5e+01)))))

(event Input|AxisEvents|InputAxisMoveForward
  (params (AxisValue :type Float%20%28single-precision%29))
  ;[1 1 1] Movement
  (Pawn|Input|AddMovementInput (Transformation|GetActorForwardVector) AxisValue false))

(event Input|AxisEvents|InputAxisMoveRight
  (params (AxisValue :type Float%20%28single-precision%29))
  ;[1 1 1] Movement
  (Pawn|Input|AddMovementInput (Transformation|GetActorRightVector) AxisValue false))

(event Input|AxisEvents|InputAxisLookRight/Left
  (params (AxisValue :type Float%20%28single-precision%29))
  ;[1 1 1] Камера
  (Pawn|Input|AddControllerYawInput AxisValue))

(fn ConstructionScript)